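; Ranged soldier enemy that chases the Lenin actor and shoots bullets at it, extending a parent class.
; Tick drives a state machine: idle picks move or attack by range, and a TaskInProgress state stops re-triggering during AI moves and attack cooldowns.
; Damage reduces Health to the Dead state, which stops movement, plays the death montage, freezes it on a notify with collision off, and sets a lifespan.
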(event Custom|Child%20Move
  (Variables|Default|SetStates "NewEnumerator0")
  (AI|AIMoveTo self "0, 0, 0" (Variables|Default|GetLenin) (- (Variables|Default|GetATK%20Range%20Radius) 1e+02) false
    (:OnSuccess
      (Variables|Default|SetStates "NewEnumerator3"))
    (:OnFail
      (Variables|Default|SetStates "NewEnumerator1"))))

(event Custom|Child%20Attack
  (Variables|Default|SetStates "NewEnumerator0")
  (Game|SpawnActorfromClass "/Game/A/AI/BP_Bullet.BP_Bullet_C" (Math|Transform|MakeTransform (Transformation|GetActorLocation) (Math|Rotator|MakeRotator 0.0 0.0 (.yaw (Math|Rotator|FindLookatRotation (Transformation|GetActorLocation) (Transformation|GetActorLocation (Variables|Default|GetLenin))))) "1,1,1") "AlwaysSpawn" 0 (Variables|Default|GetLenin) 0)
  (Utilities|FlowControl|Delay (Variables|Default|GetATK%20Cooldown))
  (Variables|Default|SetStates "NewEnumerator1"))

(event Custom|Child%20Idle
  (Variables|Default|SetStates "NewEnumerator0")
  (if (> (Math|Vector|Distance(Vector) (Transformation|GetActorLocation (Variables|Default|GetLenin)) (Transformation|GetActorLocation)) (Variables|Default|GetATK%20Range%20Radius))
    (Variables|Default|SetStates "NewEnumerator2")
    (else
      (Variables|Default|SetStates "NewEnumerator3"))))

(event Custom|Dying
  (Variables|Default|SetStates "NewEnumerator0")
  (Actor|SetLifeSpan 5.0)
  (Components|Movement|StopMovementImmediately (Variables|Character|GetCharacterMovement))
  (Variables|/Script/Engine.CharacterMovementComponent|SetMaxAcceleration (Variables|Character|GetCharacterMovement) 0.0)
  (Variables|/Script/Engine.CharacterMovementComponent|SetbOrientRotationToMovement (Variables|Character|GetCharacterMovement) false)
  (Animation|Montage|PlayMontage (Variables|Character|GetMesh) "/Game/A/AI/Soldier/AM_Soldier_Death.AM_Soldier_Death"
    (:OnNotifyBegin
      (Collision|SetCollisionEnabled (Variables|Default|GetCapsuleComponent) "NoCollision")
      (Animation|Montage|PlayMontage (Variables|Character|GetMesh) "/Game/A/AI/Soldier/AM_Soldier_Death.AM_Soldier_Death" 0.0 57.0))))

(event Game|Damage|EventAnyDamage
  (params (Damage :type Float%20%28single-precision%29) (DamageType :type Damage%20Type%20Object%20Reference) (InstigatedBy :type Controller%20Object%20Reference) (DamageCauser :type Actor%20Object%20Reference))
  (bind _output_get (Variables|Default|SetHealth (- (Variables|Default|GetHealth) Damage)))
  (if (<= _output_get 0.0)
    (Variables|Default|SetStates "NewEnumerator4")))

(event EventBeginPlay
  (|CallParentFunction)
  (Pawn|SpawnDefaultController)
  (Variables|/Script/Engine.CharacterMovementComponent|SetMaxWalkSpeed (Variables|Character|GetCharacterMovement) (Variables|Default|GetWalk%20Speed))
  (Variables|Default|SetStates "NewEnumerator1"))

(event EventTick
  (params (DeltaSeconds :type Float%20%28single-precision%29))
  (|CallParentFunction 0.0)
  (switch Utilities|FlowControl|Switch|SwitchonEnum_EnemyStates (Variables|Default|GetStates)
    (:NewEnumerator1
      (CallFunction|ChildIdle))
    (:NewEnumerator2
      (CallFunction|ChildMove))
    (:NewEnumerator3
      (CallFunction|ChildAttack))
    (:NewEnumerator4
      (CallFunction|Dying))))

(fn ConstructionScript
  (|CallParentFunction))