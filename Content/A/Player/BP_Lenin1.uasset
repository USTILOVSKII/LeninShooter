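; Player character (Lenin) for a top-down game with a cursor-targeted hammer area attack, health and death montage.
; BeginPlay shows the start menu on the StartMenu level, otherwise spawns the WaveSpawner and HUD.
; Tick moves a green/red range decal under the cursor, runs the hammer cooldown and updates bar percentages.
; In-range clicks play the hammer montage, whose notify shakes the camera and damages enemies overlapping a sphere at the clicked point.
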(event Custom|Exit
  ;[1 1 1] MenuTransitions
  (Game|QuitGame 0 "Quit" false))

(event Custom|New%20Game
  ;[1 1 1] MenuTransitions
  (Game|OpenLevel(byName) "TestMap3"))

(event Game|Damage|EventAnyDamage
  (params (Damage :type Float%20%28single-precision%29) (DamageType :type Damage%20Type%20Object%20Reference) (InstigatedBy :type Controller%20Object%20Reference) (DamageCauser :type Actor%20Object%20Reference))
  ;[1 1 1] Take Damage
  (if (not (Variables|Default|GetIsDeath))
    (Variables|PlayerStats|SetCur%20HP (- (Variables|PlayerStats|GetCur%20HP) Damage))
    (CallFunction|GetHP%)
    (if (<= (Variables|PlayerStats|GetCur%20HP) 0.0)
      (Animation|Montage|PlayMontage (Variables|Character|GetMesh) "/Game/Ilyich/Animations/M_IluyichDefeted.M_IluyichDefeted"
        (:OnNotifyBegin
          (Variables|StatesBools|SetCanMove false)
          (Variables|Default|SetIsDeath true))))))

(event EventBeginPlay
  (bind _returnvalue (Game|GetCurrentLevelName true))
  (if (Utilities|Enum|Equal(Enum) _returnvalue "StartMenu")
    (Input|DisableInput (Game|GetPlayerController 0))
    (bind _returnvalue_2 (UserInterface|CreateWidget "/Game/B/UserInterface/UI_StartMenu.UI_StartMenu_C" 0 self))
    (bind _output_get (Variables|UI|SetStartMenu _returnvalue_2))
    (UserInterface|Viewport|AddtoViewport _output_get 0)
    (else
      (Utilities|FlowControl|Sequence
        (:then_0
          (Variables|PlayerStats|SetCur%20HP (Variables|PlayerStats|GetMax%20HP))
          (CallFunction|GetHP%))
        (:then_1
          (bind _returnvalue_3 (Game|SpawnActorfromClass "/Game/A/AI/WaveSpawner.WaveSpawner_C" (Math|Transform|MakeTransform "0, 0,-1000.000000" "0, 0, 0" "1,1,1") "AlwaysSpawn" 0 self 0))
          (Variables|Default|SetWaveSpawner _returnvalue_3))
        (:then_2
          (bind _returnvalue_4 (UserInterface|CreateWidget "/Game/B/UserInterface/UI_HUD.UI_HUD_C" 0 self (Variables|Default|GetWaveSpawner)))
          (bind _output_get_2 (Variables|UI|SetUI _returnvalue_4))
          (UserInterface|Viewport|AddtoViewport _output_get_2 0))
        (:then_3
          (Input|EnableInput (Game|GetPlayerController 0)))))))

(event EventTick
  (params (DeltaSeconds :type Float%20%28single-precision%29))
  (bind _returnvalue (Game|GetPlayerController 0))
  (bind _hitresult (Game|Player|GetHitResultUnderCursorbyChannel _returnvalue "TraceTypeQuery1" true))
  (bind (_bblockinghit _binitialoverlap _time _distance _location _impactpoint _normal _impactnormal) (Collision|BreakHitResult _hitresult))
  (Utilities|FlowControl|Sequence
    (:then_0
      (if (>= (Math|Vector|Distance(Vector) _location (Transformation|GetActorLocation)) (Variables|PlayerStats|GetHammer%20ATK%20Radius))
        (Rendering|Components|Decal|SetDecalMaterial (Variables|Default|GetDecal) "/Game/A/Player/M_Cursor_Decal_Red.M_Cursor_Decal_Red")
        (Variables|StatesBools|SetInHammerRadius false)
        (else
          (Rendering|Components|Decal|SetDecalMaterial (Variables|Default|GetDecal) "/Game/A/Player/M_Cursor_Decal_Green.M_Cursor_Decal_Green")
          (Variables|StatesBools|SetInHammerRadius true)))
      (Transformation|SetWorldLocationAndRotation (Variables|Default|GetDecal) _location (Math|Rotator|MakeRotationfromAxes _impactnormal "0, 0, 0" "0, 0, 0") false false))
    (:then_1
      (if (Variables|StatesBools|GetHammerReady)
        (CallFunction|GetHammer%)
        (else
          (CallFunction|GetHammer%)
          (bind _output_get (Variables|PlayerStats|SetCurHammerCooldown (+ (Variables|PlayerStats|GetCurHammerCooldown) (Utilities|Time|GetWorldDeltaSeconds))))
          (if (>= _output_get (Variables|PlayerStats|GetMaxHammerCooldown))
            (Variables|StatesBools|SetHammerReady true)
            (Variables|PlayerStats|SetCurHammerCooldown 0.0)))))))

(event Input|ActionEvents|InputActionActionBtn1
  (params (Key :type Key%20Structure :default "None"))
  (:Pressed
    (Variables|Default|SetATKHammerLocation (.Location (Collision|BreakHitResult (.HitResult (Game|Player|GetHitResultUnderCursorbyChannel (Game|GetPlayerController 0) "TraceTypeQuery1" true)))))
    (if (Variables|StatesBools|GetInHammerRadius)
      (if (Variables|StatesBools|GetCanHammerATK)
        (if (Variables|StatesBools|GetHammerReady)
          (Variables|StatesBools|SetCanHammerATK false)
          (Variables|StatesBools|SetCanMove false)
          (Variables|StatesBools|SetHammerBarZero true)
          (CallFunction|SetRotationonMouse)
          (Animation|Montage|PlayMontage (Variables|Character|GetMesh) "/Game/A/Player/Animations/AM_HammerATK.AM_HammerATK"
            (:OnCompleted
              (Variables|StatesBools|SetCanMove true)
              (Variables|StatesBools|SetHammerReady false)
              (Variables|StatesBools|SetCanHammerATK true)
              (Variables|StatesBools|SetHammerBarZero false))
            (:OnNotifyBegin
              (Camera|PlayWorldCameraShake "/Game/B/Player/BP_Shake.BP_Shake_C" (Transformation|GetActorLocation) 0.0 1.5e+04)
              (Rendering|Debug|DrawDebugSphere (Variables|Default|GetATKHammerLocation) (Variables|Default|GetAttack%20Radius) 36 "(R=0.078458,G=0.105885,B=1.000000,A=1.000000)" 2.0 2.0)
              (bind _outactors (Collision|SphereOverlapActors (Variables|Default|GetATKHammerLocation) (Variables|Default|GetAttack%20Radius) (Utilities|Array|MakeArray "ObjectTypeQuery3") 0 (Utilities|Array|MakeArray self)))
              (for _array_element _outactors
                (CallFunction|Attack _array_element (Variables|Default|GetHammerDamage))))))))))

(event Input|AxisEvents|InputAxisMoveForward
  (params (AxisValue :type Float%20%28single-precision%29))
  ;[1 1 1] Control
  (if (Variables|StatesBools|GetCanMove)
    (Pawn|Input|AddMovementInput (Math|Vector|GetForwardVector (Class|SpringArmComponent|GetTargetRotation (Variables|MyCharacter|GetCameraBoom))) AxisValue false)))

(event Input|AxisEvents|InputAxisMoveRight
  (params (AxisValue :type Float%20%28single-precision%29))
  ;[1 1 1] Control
  (if (Variables|StatesBools|GetCanMove)
    (Pawn|Input|AddMovementInput (Math|Vector|GetRightVector (Class|SpringArmComponent|GetTargetRotation (Variables|MyCharacter|GetCameraBoom))) AxisValue false)))

(fn ConstructionScript)

(fn Attack
  (params (Actor :type Actor%20Object%20Reference) (DamageType :type Float%20%28single-precision%29))
  (bind _asbp_enemy (Utilities|Casting|CastToBP_Enemy Actor))
  (bind _returnvalue (Game|Damage|ApplyDamage _asbp_enemy DamageType 0 0))
  (Development|PrintString (Utilities|String|ToString(Float) _returnvalue)))

(fn SetRotationonMouse
  (bind _returnvalue (Transformation|GetActorRotation))
  (Transformation|SetWorldRotation (Variables|Collision|GetCapsuleComponent) (Math|Rotator|MakeRotator (.roll _returnvalue) (.pitch _returnvalue) (.yaw (Math|Rotator|FindLookatRotation (Transformation|GetActorLocation) (.Location (Collision|BreakHitResult (.HitResult (Game|Player|GetHitResultUnderCursorbyChannel (Game|GetPlayerController 0) "TraceTypeQuery1" true))))))) false false))

(fn GetHP%
  (Variables|UI|SetHP%25 (* (/ (Variables|PlayerStats|GetCur%20HP) (/ (Variables|PlayerStats|GetMax%20HP) 1e+02)) 0.01)))

(fn GetHammer%
  (if (Variables|StatesBools|GetHammerBarZero)
    (Variables|UI|SetHammer%25 0.0)
    (elif (Variables|StatesBools|GetHammerReady)
      (Variables|UI|SetHammer%25 1.0)
      (else
        (Variables|UI|SetHammer%25 (* (/ (Variables|PlayerStats|GetCurHammerCooldown) (/ (Variables|PlayerStats|GetMaxHammerCooldown) 1e+02)) 0.01))))))