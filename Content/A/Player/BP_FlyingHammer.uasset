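; BP_FlyingHammer is a thrown hammer projectile that flies out, damages enemies and returns to Lenin like a boomerang.
; Tick drives FloatingPawnMovement forward while spinning the mesh, then after a timer threshold sets Back and steers toward Lenin using a look-at rotation.
; Sphere overlaps apply damage to BP_Enemy actors, while touching Lenin on the return notifies Lenin and destroys the hammer.
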(event OnComponentBeginOverlap(Sphere)
  (params (OverlappedComponent :type Primitive%20Component%20Object%20Reference) (OtherActor :type Actor%20Object%20Reference) (OtherComp :type Primitive%20Component%20Object%20Reference) (OtherBodyIndex :type Integer) (bFromSweep :type Boolean) (SweepResult :type Hit%20Result%20Structure%20%28by%20ref%29))
  (if (== OtherActor (Variables|Default|GetLenin))
    (if (Variables|Default|GetBack)
      (Default|HammerIsBack (Variables|Default|GetLenin))
      (Actor|DestroyActor))
    (else
      (bind _asbp_enemy (Utilities|Casting|CastToBP_Enemy OtherActor))
      (Game|Damage|ApplyDamage _asbp_enemy 1e+02 0 0))))

(event EventBeginPlay
  (Audio|PlaySoundatLocation "/Game/A/Sound/Fly_hammers/Fly_Hammer_1.Fly_Hammer_1" "0, 0, 0" "0, 0, 0" 1.0 1.0 0.0 0 0 0))

(event EventTick
  (params (DeltaSeconds :type Float%20%28single-precision%29))
  (bind _output_get (Variables|Default|SetTimer (+ (Variables|Default|GetTimer) (Utilities|Time|GetWorldDeltaSeconds))))
  (if (> _output_get (Variables|Default|GetTimer_toBack))
    (Variables|Default|SetBack true)
    (Class|PawnMovementComponent|AddInputVector (Variables|Default|GetFloatingPawnMovement) (Math|Vector|GetForwardVector (Math|Rotator|FindLookatRotation (Transformation|GetWorldLocation (Variables|Default|GetSphere)) (Transformation|GetActorLocation (Variables|Default|GetLenin)))) true)
    (Transformation|AddRelativeRotation (Variables|Default|GetStaticMesh) "0, 0,10.000000" false false)
    (else
      (Class|PawnMovementComponent|AddInputVector (Variables|Default|GetFloatingPawnMovement) (Math|Vector|GetForwardVector (Transformation|GetWorldRotation (Variables|Default|GetSphere))) true)
      (Transformation|AddRelativeRotation (Variables|Default|GetStaticMesh) "0, 0,10.000000" false false))))

(fn ConstructionScript)