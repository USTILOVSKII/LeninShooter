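; Player character Lenin: moves camera-relative, fights with a hammer, takes damage and dies via montage.
; Button 1 either smashes the cursor point within range for area damage or, while button 2 aims, throws BP_FlyingHammer.
; Tick colors the cursor decal by range and recharges the hammer cooldown while it is in hand, feeding HUD percentages.
; BeginPlay shows the start menu on StartMenu, otherwise spawns the WaveSpawner and HUD.
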(event Custom|Hammer%20is%20Back
  (Rendering|SetVisibility (Variables|Default|GetStaticMesh) true false)
  (Variables|StatesBools|SetIsHammerInHand true))

(event Custom|Exit
  (Game|QuitGame 0 "Quit" false))

(event Custom|New%20Game
  (Game|OpenLevel(byName) "TestMap3"))

(event Game|Damage|EventAnyDamage
  (params (Damage :type Float%20%28single-precision%29) (DamageType :type Damage%20Type%20Object%20Reference) (InstigatedBy :type Controller%20Object%20Reference) (DamageCauser :type Actor%20Object%20Reference))
  ;[1 1 1] Take Damage
  (if (not (Variables|Default|GetIsDeath))
    (Variables|PlayerStats|SetCur%20HP (- (Variables|PlayerStats|GetCur%20HP) Damage))
    (CallFunction|GetHP%)
    (if (<= (Variables|PlayerStats|GetCur%20HP) 0.0)
      (Animation|Montage|PlayMontage (Variables|Character|GetMesh) "/Game/A/Player/Animations/AM_Death.AM_Death"
        (:OnNotifyBegin
          (Variables|StatesBools|SetCanMove false)
          (Variables|Default|SetIsDeath true))))))

(event EventBeginPlay
  (bind _returnvalue (Game|GetCurrentLevelName true))
  (if (Utilities|Enum|Equal(Enum) _returnvalue "StartMenu")
    (Input|DisableInput (Game|GetPlayerController 0))
    (bind _returnvalue_2 (UserInterface|CreateWidget "/Game/A/UserInterface/UI_StartMenu.UI_StartMenu_C" 0 self))
    (bind _output_get (Variables|UI|SetStartMenu _returnvalue_2))
    (UserInterface|Viewport|AddtoViewport _output_get 0)
    (else
      (Utilities|FlowControl|Sequence
        (:then_0
          (Variables|PlayerStats|SetCur%20HP (Variables|PlayerStats|GetMax%20HP))
          (CallFunction|GetHP%))
        (:then_1
          (bind _returnvalue_3 (Game|SpawnActorfromClass "/Game/A/AI/WaveSpawner.WaveSpawner_C" (Math|Transform|MakeTransform "0, 0,-1000.000000" "0, 0, 0" "1,1,1") "AlwaysSpawn" 0 self 0))
          (Variables|Default|SetWaveSpawner _returnvalue_3))
        (:then_2
          (bind _returnvalue_4 (UserInterface|CreateWidget "/Game/A/UserInterface/UI_HUD.UI_HUD_C" 0 self (Variables|Default|GetWaveSpawner)))
          (bind _output_get_2 (Variables|UI|SetUI _returnvalue_4))
          (UserInterface|Viewport|AddtoViewport _output_get_2 0))
        (:then_3
          (Input|EnableInput (Game|GetPlayerController 0)))))))

(event EventTick
  (params (DeltaSeconds :type Float%20%28single-precision%29))
  (bind _returnvalue (Game|GetPlayerController 0))
  (bind _capsulecomponent (Variables|Collision|GetCapsuleComponent))
  (bind _capsulecomponent_2 (Variables|Collision|GetCapsuleComponent))
  (bind _capsulecomponent_3 (Variables|Collision|GetCapsuleComponent))
  (bind _hitresult (Game|Player|GetHitResultUnderCursorbyChannel _returnvalue "TraceTypeQuery1" true))
  (bind _returnvalue_2 (Transformation|GetWorldLocation _capsulecomponent))
  (bind _returnvalue_3 (Transformation|GetWorldLocation _capsulecomponent_3))
  (bind _relativerotation (Variables|/Script/Engine.SceneComponent|GetRelativeRotation _capsulecomponent_2))
  (bind (_bblockinghit _binitialoverlap _time _distance _location _impactpoint _normal _impactnormal) (Collision|BreakHitResult _hitresult))
  (bind _returnvalue_4 (Math|Vector|GetForwardVector _relativerotation))
  (bind _returnvalue_5 (* _returnvalue_4 8e+02))
  (bind _returnvalue_6 (+ _returnvalue_3 _returnvalue_5))
  (Utilities|FlowControl|Sequence
    (:then_0
      (if (>= (Math|Vector|Distance(Vector) _location (Transformation|GetActorLocation)) (Variables|PlayerStats|GetHammer%20ATK%20Radius))
        (Rendering|Components|Decal|SetDecalMaterial (Variables|Default|GetDecal) "/Game/A/Player/M_Cursor_Decal_Red.M_Cursor_Decal_Red")
        (Variables|StatesBools|SetInHammerRadius false)
        (else
          (Rendering|Components|Decal|SetDecalMaterial (Variables|Default|GetDecal) "/Game/A/Player/M_Cursor_Decal_Green.M_Cursor_Decal_Green")
          (Variables|StatesBools|SetInHammerRadius true)))
      (Transformation|SetWorldLocationAndRotation (Variables|Default|GetDecal) _location (Math|Rotator|MakeRotationfromAxes _impactnormal "0, 0, 0" "0, 0, 0") false false))
    (:then_1
      (if (Variables|StatesBools|GetHammerReady)
        (CallFunction|GetHammer%)
        (elif (Variables|StatesBools|GetIsHammerInHand)
          (CallFunction|GetHammer%)
          (bind _output_get (Variables|PlayerStats|SetCurHammerCooldown (+ (Variables|PlayerStats|GetCurHammerCooldown) (Utilities|Time|GetWorldDeltaSeconds))))
          (if (>= _output_get (Variables|PlayerStats|GetMaxHammerCooldown))
            (Variables|StatesBools|SetHammerReady true)
            (Variables|PlayerStats|SetCurHammerCooldown 0.0)))))
    (:then_2
      (if (Variables|StatesBools|GetAiming)
        (CallFunction|SetRotationonMouse)
        (Rendering|Debug|DrawDebugLine (Math|Vector|MakeVector (.x _returnvalue_2) (.y _returnvalue_2) 3e+01) (Math|Vector|MakeVector (.x _returnvalue_6) (.y _returnvalue_6) 3e+01) "(R=1.000000,G=0.000000,B=0.000000,A=1.000000)" 0.0 1e+02)))))

(event Input|ActionEvents|InputActionActionBtn1
  (params (Key :type Key%20Structure :default "None"))
  (bind _capsulecomponent (Variables|Collision|GetCapsuleComponent))
  (bind _capsulecomponent_2 (Variables|Collision|GetCapsuleComponent))
  (bind _returnvalue (Transformation|GetWorldLocation _capsulecomponent_2))
  (bind _relativerotation (Variables|/Script/Engine.SceneComponent|GetRelativeRotation _capsulecomponent))
  (bind _returnvalue_2 (Math|Vector|GetForwardVector _relativerotation))
  (bind _returnvalue_3 (* _returnvalue_2 2e+02))
  (bind _returnvalue_4 (+ _returnvalue _returnvalue_3))
  (:Pressed
    (if (Variables|StatesBools|GetAiming)
      (if (Variables|StatesBools|GetHammerReady)
        (Variables|StatesBools|SetCanHammerATK false)
        (Variables|StatesBools|SetCanMove false)
        (Variables|StatesBools|SetHammerBarZero true)
        (Variables|StatesBools|SetNO_Anim false)
        (Animation|Montage|PlayMontage (Variables|Character|GetMesh) "/Game/A/Player/Animations/AM_HammerATK.AM_HammerATK"
          (:OnCompleted
            (Variables|StatesBools|SetNO_Anim true)
            (Variables|StatesBools|SetCanMove true)
            (Variables|StatesBools|SetHammerReady false)
            (Variables|StatesBools|SetCanHammerATK true)
            (Variables|StatesBools|SetHammerBarZero false))
          (:OnNotifyBegin
            (Variables|StatesBools|SetIsHammerInHand false)
            (Rendering|SetVisibility (Variables|Default|GetStaticMesh) false false)
            (Game|SpawnActorfromClass "/Game/A/Player/BP_FlyingHammer.BP_FlyingHammer_C" (Math|Transform|MakeTransform (Math|Vector|MakeVector (.x _returnvalue_4) (.y _returnvalue_4) 1.5e+02) _relativerotation "1,1,1") "AlwaysSpawn" 0 self 0))))
      (else
        (Variables|Default|SetATKHammerLocation (.Location (Collision|BreakHitResult (.HitResult (Game|Player|GetHitResultUnderCursorbyChannel (Game|GetPlayerController 0) "TraceTypeQuery1" true)))))
        (if (Variables|StatesBools|GetInHammerRadius)
          (if (Variables|StatesBools|GetCanHammerATK)
            (if (Variables|StatesBools|GetHammerReady)
              (if (Variables|StatesBools|GetIsHammerInHand)
                (Variables|StatesBools|SetCanHammerATK false)
                (Variables|StatesBools|SetCanMove false)
                (Variables|StatesBools|SetHammerBarZero true)
                (CallFunction|SetRotationonMouse)
                (Variables|StatesBools|SetNO_Anim false)
                (Animation|Montage|PlayMontage (Variables|Character|GetMesh) "/Game/A/Player/Animations/AM_HammerATK.AM_HammerATK"
                  (:OnCompleted
                    (Variables|StatesBools|SetNO_Anim true)
                    (Variables|StatesBools|SetCanMove true)
                    (Variables|StatesBools|SetHammerReady false)
                    (Variables|StatesBools|SetCanHammerATK true)
                    (Variables|StatesBools|SetHammerBarZero false))
                  (:OnNotifyBegin
                    (Camera|PlayWorldCameraShake "/Game/A/Player/BP_Shake.BP_Shake_C" (Transformation|GetActorLocation) 0.0 1.5e+04)
                    ;[1 1 1] PARticle
                    (Rendering|Debug|DrawDebugSphere (Variables|Default|GetATKHammerLocation) (Variables|Default|GetAttack%20Radius) 36 "(R=0.078458,G=0.105885,B=1.000000,A=1.000000)" 2.0 2.0)
                    (bind _outactors (Collision|SphereOverlapActors (Variables|Default|GetATKHammerLocation) (Variables|Default|GetAttack%20Radius) (Utilities|Array|MakeArray "ObjectTypeQuery3") 0 (Utilities|Array|MakeArray self)))
                    (for _array_element _outactors
                      (CallFunction|Attack _array_element (Variables|Default|GetHammerDamage)))))))))))))

(event Input|ActionEvents|InputActionActionBtn2
  (params (Key :type Key%20Structure :default "None"))
  (:Pressed
    (Variables|StatesBools|SetCanMove false)
    (Variables|StatesBools|SetAiming true)
    (Variables|StatesBools|SetCanHammerATK false)
    (Rendering|SetVisibility (Variables|Default|GetDecal) false false))
  (:Released
    (Variables|StatesBools|SetCanMove true)
    (Variables|StatesBools|SetAiming false)
    (Variables|StatesBools|SetCanHammerATK true)
    (Rendering|SetVisibility (Variables|Default|GetDecal) true false)))

(event Input|AxisEvents|InputAxisMoveForward
  (params (AxisValue :type Float%20%28single-precision%29))
  (if (Variables|StatesBools|GetCanMove)
    (if (Variables|StatesBools|GetNO_Anim)
      (Pawn|Input|AddMovementInput (Math|Vector|GetForwardVector (Class|SpringArmComponent|GetTargetRotation (Variables|MyCharacter|GetCameraBoom))) AxisValue false))))

(event Input|AxisEvents|InputAxisMoveRight
  (params (AxisValue :type Float%20%28single-precision%29))
  (if (Variables|StatesBools|GetCanMove)
    (if (Variables|StatesBools|GetNO_Anim)
      (Pawn|Input|AddMovementInput (Math|Vector|GetRightVector (Class|SpringArmComponent|GetTargetRotation (Variables|MyCharacter|GetCameraBoom))) AxisValue false))))

(fn ConstructionScript)

(fn Attack
  (params (Actor :type Actor%20Object%20Reference) (DamageType :type Float%20%28single-precision%29))
  (bind _asbp_enemy (Utilities|Casting|CastToBP_Enemy Actor))
  (Game|Damage|ApplyDamage _asbp_enemy DamageType 0 0))

(fn SetRotationonMouse
  (bind _capsulecomponent (Variables|Collision|GetCapsuleComponent))
  (bind _returnvalue (Transformation|GetWorldRotation _capsulecomponent))
  (Transformation|SetWorldRotation (Variables|Collision|GetCapsuleComponent) (Math|Rotator|MakeRotator (.roll _returnvalue) (.pitch _returnvalue) (.yaw (Math|Rotator|FindLookatRotation (Transformation|GetWorldLocation (Variables|Collision|GetCapsuleComponent)) (.Location (Collision|BreakHitResult (.HitResult (Game|Player|GetHitResultUnderCursorbyChannel (Game|GetPlayerController 0) "TraceTypeQuery1" true))))))) false false))

(fn GetHP%
  (Variables|UI|SetHP%25 (* (/ (Variables|PlayerStats|GetCur%20HP) (/ (Variables|PlayerStats|GetMax%20HP) 1e+02)) 0.01)))

(fn GetHammer%
  (if (Variables|StatesBools|GetHammerBarZero)
    (Variables|UI|SetHammer%25 0.0)
    (elif (Variables|StatesBools|GetHammerReady)
      (Variables|UI|SetHammer%25 1.0)
      (else
        (Variables|UI|SetHammer%25 (* (/ (Variables|PlayerStats|GetCurHammerCooldown) (/ (Variables|PlayerStats|GetMaxHammerCooldown) 1e+02)) 0.01))))))

(fn SetRotationonMouse0
  (bind _returnvalue (Transformation|GetActorRotation))
  (Transformation|SetWorldRotation (Variables|Collision|GetCapsuleComponent) (Math|Rotator|MakeRotator (.roll _returnvalue) (.pitch _returnvalue) (.yaw (Math|Rotator|FindLookatRotation (Transformation|GetActorLocation) (.Location (Collision|BreakHitResult (.HitResult (Game|Player|GetHitResultUnderCursorbyChannel (Game|GetPlayerController 0) "TraceTypeQuery1" true))))))) false false))