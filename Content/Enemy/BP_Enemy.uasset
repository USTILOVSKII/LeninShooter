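; Enemy character that chases the Lenin target and shoots at it from range.
; A Tick-driven enum state machine picks MoveTo or Attack by distance to Lenin, with TaskInProgress blocking re-entry during latent actions.
; MoveTo runs AIMoveTo to just inside attack range, then attacks on success or re-decides on failure.
; Attack spawns a BP_Bullet yawed toward Lenin, waits out the cooldown, then re-decides.
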(event Custom|Move%20To
  (Variables|Default|SetStates "NewEnumerator0")
  (AI|AIMoveTo self "0, 0, 0" (Variables|Default|GetLenin) (- (Variables|Default|GetATK%20Range%20Radius) 1e+02) false
    (:OnSuccess
      (Variables|Default|SetStates "NewEnumerator3"))
    (:OnFail
      (Variables|Default|SetStates "NewEnumerator1"))))

(event Custom|Attack
  (Variables|Default|SetStates "NewEnumerator0")
  (Game|SpawnActorfromClass "/Game/Enemy/BP_Bullet.BP_Bullet_C" (Math|Transform|MakeTransform (Transformation|GetActorLocation) (Math|Rotator|MakeRotator 0.0 0.0 (.yaw (Math|Rotator|FindLookatRotation (Transformation|GetActorLocation) (Transformation|GetActorLocation (Variables|Default|GetLenin))))) "1,1,1") "AlwaysSpawn" 0 (Variables|Default|GetLenin) 0)
  (Utilities|FlowControl|Delay (Variables|Default|GetATK%20Cooldown))
  (Variables|Default|SetStates "NewEnumerator1"))

(event Custom|Idle%20Desicion
  (Variables|Default|SetStates "NewEnumerator0")
  (if (> (Math|Vector|Distance(Vector) (Transformation|GetActorLocation (Variables|Default|GetLenin)) (Transformation|GetActorLocation)) (Variables|Default|GetATK%20Range%20Radius))
    (Variables|Default|SetStates "NewEnumerator2")
    (else
      (Variables|Default|SetStates "NewEnumerator3"))))

(event EventBeginPlay
  (Pawn|SpawnDefaultController)
  (Variables|/Script/Engine.CharacterMovementComponent|SetMaxWalkSpeed (Variables|Character|GetCharacterMovement) (Variables|Default|GetWalk%20Speed))
  (Variables|Default|SetStates "NewEnumerator1"))

(event EventTick
  (params (DeltaSeconds :type Float%20%28single-precision%29))
  (switch Utilities|FlowControl|Switch|SwitchonEnum_EnemyStates (Variables|Default|GetStates)
    (:NewEnumerator1
      (CallFunction|IdleDesicion))
    (:NewEnumerator2
      (CallFunction|Moveto))
    (:NewEnumerator3
      (CallFunction|Attack))))

(fn ConstructionScript)