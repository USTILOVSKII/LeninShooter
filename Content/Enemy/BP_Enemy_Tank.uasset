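; Enemy tank Blueprint that provides functions to animate the wheels on each side of the vehicle.
; LeftForward, LeftBackward, RIghtForward and RIghtBackward each add a TurnSpeed roll rotation to their side's five wheel components, with the sign mirrored between left and right.
; The functions are not called within this graph, and BeginPlay, Tick and the construction script only defer to the parent class.
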(event EventBeginPlay
  (|CallParentFunction) ; This node is disabled and will not be called.\nDrag off pins to build functionality.
)

(event EventTick
  (params (DeltaSeconds :type Float%20%28single-precision%29))
  (|CallParentFunction DeltaSeconds))

(fn ConstructionScript
  (|CallParentFunction))

(fn LeftForward
  (Transformation|AddRelativeRotation (Variables|Default|GetLeft1) (Math|Rotator|MakeRotator (Variables|Default|GetTurnSpeed) 0.0 0.0) false false)
  (Transformation|AddRelativeRotation (Variables|Default|GetLeft2) (Math|Rotator|MakeRotator (Variables|Default|GetTurnSpeed) 0.0 0.0) false false)
  (Transformation|AddRelativeRotation (Variables|Default|GetLeft3) (Math|Rotator|MakeRotator (Variables|Default|GetTurnSpeed) 0.0 0.0) false false)
  (Transformation|AddRelativeRotation (Variables|Default|GetLeft4) (Math|Rotator|MakeRotator (Variables|Default|GetTurnSpeed) 0.0 0.0) false false)
  (Transformation|AddRelativeRotation (Variables|Default|GetLeft5) (Math|Rotator|MakeRotator (Variables|Default|GetTurnSpeed) 0.0 0.0) false false))

(fn LeftBackward
  (Transformation|AddRelativeRotation (Variables|Default|GetLeft1) (Math|Rotator|MakeRotator (* (Variables|Default|GetTurnSpeed) -1.0) 0.0 0.0) false false)
  (Transformation|AddRelativeRotation (Variables|Default|GetLeft2) (Math|Rotator|MakeRotator (* (Variables|Default|GetTurnSpeed) -1.0) 0.0 0.0) false false)
  (Transformation|AddRelativeRotation (Variables|Default|GetLeft3) (Math|Rotator|MakeRotator (* (Variables|Default|GetTurnSpeed) -1.0) 0.0 0.0) false false)
  (Transformation|AddRelativeRotation (Variables|Default|GetLeft4) (Math|Rotator|MakeRotator (* (Variables|Default|GetTurnSpeed) -1.0) 0.0 0.0) false false)
  (Transformation|AddRelativeRotation (Variables|Default|GetLeft5) (Math|Rotator|MakeRotator (* (Variables|Default|GetTurnSpeed) -1.0) 0.0 0.0) false false))

(fn RIghtForward
  (Transformation|AddRelativeRotation (Variables|Default|GetRight1) (Math|Rotator|MakeRotator (* (Variables|Default|GetTurnSpeed) -1.0) 0.0 0.0) false false)
  (Transformation|AddRelativeRotation (Variables|Default|GetRight2) (Math|Rotator|MakeRotator (* (Variables|Default|GetTurnSpeed) -1.0) 0.0 0.0) false false)
  (Transformation|AddRelativeRotation (Variables|Default|GetRight3) (Math|Rotator|MakeRotator (* (Variables|Default|GetTurnSpeed) -1.0) 0.0 0.0) false false)
  (Transformation|AddRelativeRotation (Variables|Default|GetRight4) (Math|Rotator|MakeRotator (* (Variables|Default|GetTurnSpeed) -1.0) 0.0 0.0) false false)
  (Transformation|AddRelativeRotation (Variables|Default|GetRight5) (Math|Rotator|MakeRotator (* (Variables|Default|GetTurnSpeed) -1.0) 0.0 0.0) false false))

(fn RIghtBackward
  (Transformation|AddRelativeRotation (Variables|Default|GetRight1) (Math|Rotator|MakeRotator (Variables|Default|GetTurnSpeed) 0.0 0.0) false false)
  (Transformation|AddRelativeRotation (Variables|Default|GetRight2) (Math|Rotator|MakeRotator (Variables|Default|GetTurnSpeed) 0.0 0.0) false false)
  (Transformation|AddRelativeRotation (Variables|Default|GetRight3) (Math|Rotator|MakeRotator (Variables|Default|GetTurnSpeed) 0.0 0.0) false false)
  (Transformation|AddRelativeRotation (Variables|Default|GetRight4) (Math|Rotator|MakeRotator (Variables|Default|GetTurnSpeed) 0.0 0.0) false false)
  (Transformation|AddRelativeRotation (Variables|Default|GetRight5) (Math|Rotator|MakeRotator (Variables|Default|GetTurnSpeed) 0.0 0.0) false false))